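; Player camera that spawns and follows a physics ball and handles turn-based, putting-style launches.
; Holding LaunchBall oscillates a clamped power meter; releasing sets the ball's velocity along the camera's forward direction, constrained to the ground plane.
; Tick smoothly moves the spring arm to the ball, prints debug values and opens a new turn once the ball slows below a speed threshold.
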(event `InputAction|LaunchBall`
  (params (Key :type "Key Structure" :default "AnyKey"))
  (bind _isnewturn (`self.IsNewTurn`))
  (:`Pressed`
    (if _isnewturn
      (set `self.IsLaunchPressed` true)))
  (:`Released`
    (if _isnewturn
      (set `self.IsLaunchPressed` false)
      (`PrimitiveComponent.SetAllPhysicsLinearVelocity` (`StaticMeshActor.StaticMeshComponent` (stale `self.ReceiveBeginPlay` _returnvalue)) (+ (* (`KismetMathLibrary.Conv_RotatorToVector` (`KismetMathLibrary.MakeRotFromZX` (`self.UpVectorWS`) (`SceneComponent.GetForwardVector` (`self.Camera`)))) (* (`self.BallLaunchMultiplier`) (`self.BallLaunchAmount`))) (`self.GetVelocity` (stale `self.ReceiveBeginPlay` _returnvalue))) false)
      (set `self.BallLaunchMultiplier` 0.0)
      (set `self.IsNewTurn` false))))

(event `self.ReceiveBeginPlay`
  ;[1 1 1] Spawn Ball Actor
  (bind _returnvalue (`|SpawnActorFromClass` "/Game/Blueprints/BP_PhysicsBall.BP_PhysicsBall_C" (`SceneComponent.K2_GetComponentToWorld` (`self.SpringArm`)) "Undefined" "OverrideRootScale")))

(event `self.ReceiveTick`
  (params (DeltaSeconds :type "Float (single-precision)"))
  (bind _springarm (`self.SpringArm`))
  ;[1 1 1] Make Camera Follow Ball
  (`SceneComponent.K2_SetWorldLocation` _springarm (`KismetMathLibrary.VInterpTo` (`SceneComponent.K2_GetComponentLocation` _springarm) (`SceneComponent.K2_GetComponentLocation` (`StaticMeshActor.StaticMeshComponent` (stale `self.ReceiveBeginPlay` _returnvalue))) DeltaSeconds 25.0) true true)
  (bind _returnvalue (`KismetMathLibrary.VSize` (`self.GetVelocity` (stale `self.ReceiveBeginPlay` _returnvalue))))
  (`KismetSystemLibrary.PrintString` (`KismetStringLibrary.Conv_DoubleToString` _returnvalue))
  (if (`self.IsNewTurn`)
    (if (`self.IsLaunchPressed`)
      (bind _output_get (set `self.BallLaunchMultiplier` (`KismetMathLibrary.FClamp` (+ (`self.BallLaunchMultiplier`) (* (`self.BallLaunchAddOrRemove`) (`GameplayStatics.GetWorldDeltaSeconds`))) 0.0 3.0)))
      (`KismetSystemLibrary.PrintString` (`KismetStringLibrary.Conv_DoubleToString` _output_get))
      (if (>= (`self.BallLaunchMultiplier`) 3.0)
        (set `self.BallLaunchAddOrRemove` -1)
        (elif (<= (`self.BallLaunchMultiplier`) 0.0)
          (set `self.BallLaunchAddOrRemove` 1))))
    (elif (<= _returnvalue (`self.NewTurnSpeedThreshold`))
      (set `self.IsNewTurn` true))))

(fn `UserConstructionScript`)