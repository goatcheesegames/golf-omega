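; Backup of the player camera Blueprint, which spawns a physics ball, follows it and lets the player launch it.
; BeginPlay spawns the ball at the spring arm, and Tick eases the arm toward the ball's mesh with interpolation and sweep.
; LaunchBall adds a scaled impulse-like velocity to the ball's current velocity, along camera forward flattened perpendicular to UpVectorWS.
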(event `InputAction|LaunchBall`
  (params (Key :type "Key Structure" :default "AnyKey"))
  (:`Pressed`
    (`PrimitiveComponent.SetAllPhysicsLinearVelocity` (`StaticMeshActor.StaticMeshComponent` (stale `self.ReceiveBeginPlay` _returnvalue)) (+ (* (`KismetMathLibrary.Conv_RotatorToVector` (`KismetMathLibrary.MakeRotFromZX` (`self.UpVectorWS`) (`SceneComponent.GetForwardVector` (`self.Camera`)))) (`self.BallLaunchAmount`)) (`self.GetVelocity` (stale `self.ReceiveBeginPlay` _returnvalue))) false)))

(event `self.ReceiveBeginPlay`
  (bind _returnvalue (`|SpawnActorFromClass` "/Game/Blueprints/BP_PhysicsBall.BP_PhysicsBall_C" (`SceneComponent.K2_GetComponentToWorld` (`self.SpringArm`)) "Undefined" "OverrideRootScale")))

(event `self.ReceiveTick`
  (params (DeltaSeconds :type "Float (single-precision)"))
  (bind _springarm (`self.SpringArm`))
  (`SceneComponent.K2_SetWorldLocation` _springarm (`KismetMathLibrary.VInterpTo` (`SceneComponent.K2_GetComponentLocation` _springarm) (`SceneComponent.K2_GetComponentLocation` (`StaticMeshActor.StaticMeshComponent` (stale `self.ReceiveBeginPlay` _returnvalue))) DeltaSeconds 10.0) true true))

(fn `UserConstructionScript`)